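; Base player class for a multiplayer game, handling attack and ability input, health, mana, death and respawn.
; Input calls server events when the player is alive and not attacking; their bodies are empty for child classes to override.
; Damage updates the stats struct, health UI and voice sounds; death freezes movement, then after a delay the controller is messaged to deduct a life and respawn, and this actor is destroyed.
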(event `Server_PrimarryAttack`
  ;[1 1 1] Attack overrides
)

(event `Server_Ability1`
  ;[1 1 1] Attack overrides
)

(event `Server_Ability2`
  ;[1 1 1] Attack overrides
)

(event `Server_Ability3`
  ;[1 1 1] Attack overrides
)

(event `InputAction|PrimarryAttack`
  (params (Key :type "Key Structure"))
  (:`Pressed`
    (if (not (`self.IsDead?`))
      (if (not (`self.CurrentlyAttacking`))
        (`self.Server_PrimarryAttack`)))))

(event `InputAction|Ability1`
  (params (Key :type "Key Structure"))
  (:`Pressed`
    (if (not (`self.IsDead?`))
      (if (not (`self.CurrentlyAttacking`))
        (`self.Server_Ability1`)))))

(event `Server_KillPlayer`
  (if (not (`self.IsDead?`))
    (set `self.IsDead?` true)
    (`self.Multi_PlayerDeath`)
    (message `/Game/_Main/Interfaces/INT_PlayerController.MovementFrozen` (`self.ControllerRef`) true)
    (`KismetSystemLibrary.Delay` 5.0)
    (`self.ServerRespondPlayer`)))

(event `InputAction|Ability2`
  (params (Key :type "Key Structure"))
  (:`Pressed`
    (if (not (`self.IsDead?`))
      (if (not (`self.CurrentlyAttacking`))
        (`self.Server_Ability2`)))))

(event `InputAction|Ability3`
  (params (Key :type "Key Structure"))
  (:`Pressed`
    (if (not (`self.IsDead?`))
      (if (not (`self.CurrentlyAttacking`))
        (`self.Server_Ability3`)))))

(event `self.ReceiveAnyDamage`
  (params (Damage :type "Float (single-precision)") (DamageType :type "DamageType Object Reference") (InstigatedBy :type "Controller Object Reference") (DamageCauser :type "Actor Object Reference"))
  ;[1 1 1] Damage Event
  (bind _structout (setmembers `/Game/_Main/S_Stats` :`StructRef` (`self.Stats`) :`CurrentHealth` (- (`.CurrentHealth_2_48A2398F46E20091E1F642AC1BB520C7` (break `/Game/_Main/S_Stats` (`self.Stats`))) Damage)))
  (`self.Client_UpdateHealthUi` (`.CurrentHealth_2_48A2398F46E20091E1F642AC1BB520C7` (break `/Game/_Main/S_Stats` _structout)))
  (`self.Multi_VoiceSounds` (`self.VoicePain`) (`self.K2_GetActorLocation`))
  (if (<= (`.CurrentHealth_2_48A2398F46E20091E1F642AC1BB520C7` (break `/Game/_Main/S_Stats` (`self.Stats`))) 0.0)
    (`self.Server_KillPlayer`)
    (`self.Multi_VoiceSounds` (`self.VoiceDeath`) (`self.K2_GetActorLocation`))))

(event `ServerRespondPlayer`
  (bind _controllerref (`self.ControllerRef`))
  (message `/Game/_Main/Interfaces/INT_PlayerController.DecreaseLives` _controllerref)
  (bind _structout (setmembers `/Game/_Main/S_Stats` :`StructRef` (`self.Stats`)))
  (bind ((`MaxHealth_4_E022879F47CF69107432B58A8C2983C5` _maxhealth) (`MaxMana_8_B681D640491923A476C3B79370DC2457` _maxmana)) (break `/Game/_Main/S_Stats` _structout))
  (`self.Client_UpdateHealthUi` _maxhealth)
  (`self.Client_UpdateManaUi` _maxmana)
  (message `/Game/_Main/Interfaces/INT_PlayerController.PlayerRespawn` _controllerref (`self.f_GetSpawnedLocation`) (`self.PlayerClas`))
  (`KismetSystemLibrary.Delay` 0.2)
  (`self.K2_DestroyActor`))

(event `Client_UpdateHealthUi`
  (params (CurrentHealth :type "Float (double-precision)"))
  (message `/Game/_Main/Interfaces/INT_PlayerController.UpdateHealthUI` (`self.ControllerRef`) CurrentHealth))

(event `Client_UpdateManaUi`
  (params (CurrentMana :type "Float (double-precision)"))
  (message `/Game/_Main/Interfaces/INT_PlayerController.UpdateManaUI` (`self.ControllerRef`) CurrentMana))

(event `update player movement`
  (params (state :type Boolean))
  (if state
    (message `/Game/_Main/Interfaces/INT_PlayerController.MovementFrozen` (`self.ControllerRef`) true)
    (elif (not (`self.IsDead?`))
      (message `/Game/_Main/Interfaces/INT_PlayerController.MovementFrozen` (`self.ControllerRef`) false))))

(fn `f_UpdateMana`
  (params (ManaCost :type "Float (double-precision)"))
  (returns (currentMana :type "Float (double-precision)"))
  (bind _stats (`self.Stats`))
  (bind _structout (setmembers `/Game/_Main/S_Stats` :`StructRef` _stats :`CurrentMana` (- (`.CurrentMana_6_2B652CCA4F14B2424E899AB9F1EC7BD7` (break `/Game/_Main/S_Stats` _stats)) ManaCost)))
  (return (`.CurrentMana_6_2B652CCA4F14B2424E899AB9F1EC7BD7` (break `/Game/_Main/S_Stats` _structout))))

(fn `GetPlayerStats`
  (returns (PlayerStats :type "/Game/_Main/S_Stats Structure"))
  (return (`self.Stats`)))

(fn `IsPlayerImmune`
  (returns (State :type Boolean))
  (return (`self.IsImmune`)))

(fn `PlayerDeathState`
  (returns (State :type Boolean))
  (return (`self.IsDead?`)))

(fn `UserConstructionScript`)