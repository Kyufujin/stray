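; Player controller for the dungeon game that drives pawn movement, tracks lives and handles respawning.
; Forward and right axis inputs move the cached pawn relative to control rotation unless a freeze interface event has set the stunned flag.
; Respawn spawns the supplied class slightly above the given location, possesses it and clears the stun, or prints Game Over once lives drop below zero.
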(event `self.ReceiveBeginPlay`
  (set `self.PlayerPawn` (`self.K2_GetPawn`)))

(event `/Game/_Main/Interfaces/INT_PlayerController.MovementFrozen`
  (params (State :type Boolean))
  ;[1 1 1] Interfaces
  (set `self.PlayerStunned` State))

(event `InputAxis|MoveForward`
  (params (AxisValue :type "Float (single-precision)"))
  ;[1 1 1] Multiplayer character movement
  (`self.PlayerPawn`
    (:`then`
      (if (not (`self.PlayerStunned`))
        (`Pawn.AddMovementInput` (`self.PlayerPawn`) (`KismetMathLibrary.GetForwardVector` (`self.GetControlRotation`)) AxisValue false)))
    (:`else`)))

(event `/Game/_Main/Interfaces/INT_PlayerController.IncreaseLives`
  ;[1 1 1] Interfaces
  (set `self.PlayerLives` (+ (`self.PlayerLives`) 1)))

(event `/Game/_Main/Interfaces/INT_PlayerController.DecreaseLives`
  ;[1 1 1] Interfaces
  (set `self.PlayerLives` (- (`self.PlayerLives`) 1)))

(event `InputAxis|MoveRight`
  (params (AxisValue :type "Float (single-precision)"))
  ;[1 1 1] Multiplayer character movement
  (`self.PlayerPawn`
    (:`then`
      (if (not (`self.PlayerStunned`))
        (`Pawn.AddMovementInput` (`self.PlayerPawn`) (`KismetMathLibrary.GetRightVector` (`self.GetControlRotation`)) AxisValue false)))
    (:`else`)))

(event `/Game/_Main/Interfaces/INT_PlayerController.PlayerRespawn`
  (params (SpawnLocation :type "Vector Structure") (PlayerCllass :type "/Game/_Main/BP_PlayerBase Class Reference"))
  (if (>= (`self.PlayerLives`) 0)
    (bind _returnvalue (`|SpawnActorFromClass` PlayerCllass (`KismetMathLibrary.MakeTransform` (+ SpawnLocation (0.0 0.0 150.0))) "AlwaysSpawn" "OverrideRootScale" null null))
    (`self.Possess` _returnvalue)
    (set `self.PlayerStunned` false)
    (set `self.PlayerPawn` (`self.K2_GetPawn`))
    (else
      (`KismetSystemLibrary.PrintString` "Game Over"))))

(fn `UserConstructionScript`)